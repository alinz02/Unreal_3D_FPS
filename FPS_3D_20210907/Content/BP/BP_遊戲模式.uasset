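; BP_遊戲模式 is a game mode Blueprint that runs a minute-and-second countdown (分 and 秒).
; Tick feeds a one-second Delay that decrements the seconds, wrapping them to 59 and borrowing from the minutes.
; When no minutes remain, it resets the seconds to zero and calls SetGamePaused with false, although its comment says the game pauses.
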(event `self.ReceiveTick`
  (params (DeltaSeconds :type "Float (single-precision)"))
  ;[1 0.1927 0.1927] 倒數系統
  ;;[1 1 1] 每秒秒數-1
  (`KismetSystemLibrary.Delay` 1.0)
  (bind _output_get (set `self.秒` (- (`self.秒`) 1)))
  ;;[1 1 1] 秒數<0回到59
  (if (< _output_get 0)
    (set `self.秒` 59)
    ;;[1 1 1] 分>0時 分-1
    (if (> (`self.分`) 0)
      (set `self.分` (- (`self.分`) 1))
      (else
        ;;[1 1 1] 秒設為0並暫停遊戲
        (if (== (`self.秒`) 59)
          (set `self.秒` 0)
          (`GameplayStatics.SetGamePaused` false))))))

(fn `UserConstructionScript`)